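; Destruction_BP is a destructible actor with a box trigger that, as wired, only adds 10 to its Damage variable when FirstPersonCharacter overlaps it.
; BeginPlay starts a looping one-second LightTimer, whose handler is empty.
; Unconnected nodes hold the intended effects: a random point light colour with a timer clear, and radius damage to the Destructible at the impact point with a sound.
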(event OnComponentBeginOverlap(Box)
  (params (OverlappedComponent :type Primitive%20Component%20Object%20Reference) (OtherActor :type Actor%20Object%20Reference) (OtherComp :type Primitive%20Component%20Object%20Reference) (OtherBodyIndex :type Integer) (bFromSweep :type Boolean) (SweepResult :type Hit%20Result%20Structure%20%28by%20ref%29))
  (Utilities|Casting|CastToFirstPersonCharacter OtherActor)
  (Variables|Default|SetDamage (+ (Variables|Default|GetDamage) 1e+01)))

(event Custom|LightTimer)

(event EventBeginPlay
  (Utilities|Time|SetTimerbyFunctionName 0 "LightTimer" 1.0 true))

(fn ConstructionScript)