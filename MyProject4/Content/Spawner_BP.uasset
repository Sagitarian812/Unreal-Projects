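; Spawner Blueprint that fills a volume with Hover_BP actors, switched on and off by the first-person character.
; Successive character overlaps with the Box trigger alternate via FlipFlop between starting a looping one-second Spawn timer and clearing it, destroying all tracked actors.
; Spawn places each actor at a random point inside SpawnVolume and appends it to SpawnedActor, which is never emptied.
; The construction script sizes SpawnVolume from BoxExtent.
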(event OnComponentBeginOverlap(Box)
  (params (OverlappedComponent :type Primitive%20Component%20Object%20Reference) (OtherActor :type Actor%20Object%20Reference) (OtherComp :type Primitive%20Component%20Object%20Reference) (OtherBodyIndex :type Integer) (bFromSweep :type Boolean) (SweepResult :type Hit%20Result%20Structure%20%28by%20ref%29))
  (Utilities|Casting|CastToFirstPersonCharacter OtherActor)
  (Utilities|FlowControl|FlipFlop
    (:A
      (Utilities|Time|SetTimerbyFunctionName 0 "Spawn" 1.0 true))
    (:B
      (Utilities|Time|ClearTimerbyFunctionName 0 "Spawn")
      (for _array_element (Variables|Default|GetSpawnedActor)
        (Actor|DestroyActor _array_element)))))

(event Custom|Spawn
  (bind _returnvalue (Game|SpawnActorfromClass "/Game/Hover_BP.Hover_BP_C" (Math|Transform|MakeTransform (Math|Random|RandomPointinBoundingBox (Transformation|GetWorldLocation (Variables|Default|GetSpawnVolume)) (Variables|Default|GetBox%20Extent)) "0, 0, 0" "1,1,1") "Undefined" 0 0))
  (Utilities|Array|Add (Variables|Default|GetSpawnedActor) _returnvalue))

(fn ConstructionScript
  (Components|Box|SetBoxExtent (Variables|Default|GetSpawnVolume) (Variables|Default|GetBox%20Extent) true))